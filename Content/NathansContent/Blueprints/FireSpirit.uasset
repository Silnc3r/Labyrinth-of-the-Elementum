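; FireSpirit is an enemy pawn that wanders, chases when it sees a pawn, and burns the TopDownCharacter on contact.
; PawnSensing starts an AI move targeting player controller 0, and a retriggerable delay times out sensing.
; Tick uses delays to drop the chase and roam to random reachable points.
; Box overlap deals an instant hit, then Tick applies timed burn damage up to MaxTimes, with BeenHit clearing shortly after overlap ends.
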(event `self.ReceiveBeginPlay`)

(event `self.PawnSensing.OnSeePawn`
  (params (Pawn :type "Pawn Object Reference"))
  (`|ExecutionSequence`
    (:`then_0`
      (set `self.IsSensingPawn` true)
      (set `self.IsChasing` true)
      (`|AIMoveTo` self (0.0 0.0 0.0) (`GameplayStatics.GetPlayerController` 0)))
    (:`then_1`
      (`KismetSystemLibrary.RetriggerableDelay` 0.6)
      (set `self.IsSensingPawn` false))))

(event `self.ReceiveTick`
  (params (DeltaSeconds :type "Float (single-precision)"))
  (`|ExecutionSequence`
    (:`then_0`
      (if (not (`self.IsSensingPawn`))
        (`KismetSystemLibrary.Delay` 0.4)
        (if (not (`self.IsSensingPawn`))
          (set `self.IsChasing` false))))
    (:`then_1`
      (if (not (`self.IsChasing`))
        (`KismetSystemLibrary.Delay` (`KismetMathLibrary.RandomFloatInRange` 2.0 5.0))
        (`|AIMoveTo` self (`NavigationSystemV1.K2_GetRandomReachablePointInRadius` (`self.K2_GetActorLocation`) 1500.0 null null) null)))
    (:`then_2`
      (if (`self.TakenDamage`)
        (if (== (`self.Times`) (`self.MaxTimes`))
          (set `self.TakenDamage` false)
          (set `self.Times` 0.0)
          (else
            (bind _astop_down_character (cast `/Game/2DTopDownControllerStuff/TopDownCharacter` (stale `self.Box.OnComponentBeginOverlap` OtherActor)))
            (`KismetSystemLibrary.Delay` 1.0)
            (set `/Game/2DTopDownControllerStuff/TopDownCharacter.Health` (- (`/Game/2DTopDownControllerStuff/TopDownCharacter.Health` _astop_down_character) 1.0) _astop_down_character)
            (set `self.Times` (+ (`self.Times`) 1.0))))))))

(event `self.Box.OnComponentBeginOverlap`
  (params (OverlappedComponent :type "PrimitiveComponent Object Reference") (OtherActor :type "Actor Object Reference") (OtherComp :type "PrimitiveComponent Object Reference") (OtherBodyIndex :type Integer) (bFromSweep :type Boolean) (SweepResult :type "HitResult Structure (by ref)"))
  (if (not (`self.Been hit`))
    (bind _astop_down_character (cast `/Game/2DTopDownControllerStuff/TopDownCharacter` OtherActor))
    (set `/Game/2DTopDownControllerStuff/TopDownCharacter.Health` (- (`/Game/2DTopDownControllerStuff/TopDownCharacter.Health` _astop_down_character) 10.0) _astop_down_character)
    (set `self.Times` 0.0)
    (set `self.TakenDamage` true)
    (set `self.Been hit` true)))

(event `self.Box.OnComponentEndOverlap`
  (params (OverlappedComponent :type "PrimitiveComponent Object Reference") (OtherActor :type "Actor Object Reference") (OtherComp :type "PrimitiveComponent Object Reference") (OtherBodyIndex :type Integer))
  (cast `/Game/2DTopDownControllerStuff/TopDownCharacter` OtherActor)
  (`KismetSystemLibrary.Delay` 2.0)
  (set `self.Been hit` false))

(fn `UserConstructionScript`)