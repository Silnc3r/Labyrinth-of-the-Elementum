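; Trap spawner actor that keeps releasing randomly chosen cars at its Arrow component's transform.
; Tick feeds a random-length Delay, which ignores calls while counting down and so acts as a repeating timer of a few seconds.
; After each delay, a random integer runs through a branch chain to pick one of five car classes, spawned regardless of collisions.
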(event `self.ReceiveTick`
  (params (DeltaSeconds :type "Float (single-precision)"))
  (`KismetSystemLibrary.Delay` (`KismetMathLibrary.RandomFloatInRange` 2.0 10.0))
  (set `self.SpawnCar` (`KismetMathLibrary.Conv_IntToDouble` (`KismetMathLibrary.RandomIntegerInRange` 1 5)))
  (if (== (`self.SpawnCar`) 1.0)
    (`|SpawnActorFromClass` "/Game/NathansContent/Blueprints/Traps/Car.Car_C" (`SceneComponent.K2_GetComponentToWorld` (`self.Arrow`)) "AlwaysSpawn" "OverrideRootScale" null null)
    (elif (== (`self.SpawnCar`) 2.0)
      (`|SpawnActorFromClass` "/Game/NathansContent/Blueprints/Traps/Car1.Car1_C" (`SceneComponent.K2_GetComponentToWorld` (`self.Arrow`)) "AlwaysSpawn" "OverrideRootScale" null null)
      (elif (== (`self.SpawnCar`) 3.0)
        (`|SpawnActorFromClass` "/Game/NathansContent/Blueprints/Traps/Car2.Car2_C" (`SceneComponent.K2_GetComponentToWorld` (`self.Arrow`)) "AlwaysSpawn" "OverrideRootScale" null null)
        (elif (== (`self.SpawnCar`) 4.0)
          (`|SpawnActorFromClass` "/Game/NathansContent/Blueprints/Traps/Car3.Car3_C" (`SceneComponent.K2_GetComponentToWorld` (`self.Arrow`)) "AlwaysSpawn" "OverrideRootScale" null null)
          (elif (== (`self.SpawnCar`) 5.0)
            (`|SpawnActorFromClass` "/Game/NathansContent/Blueprints/Traps/Car4.Car4_C" (`SceneComponent.K2_GetComponentToWorld` (`self.Arrow`)) "AlwaysSpawn" "OverrideRootScale" null null)))))))

(fn `UserConstructionScript`)