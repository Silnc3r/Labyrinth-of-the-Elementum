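; FireJet is a trap that sprays fire while a TopDownCharacter stands inside its Box trigger.
; Box overlap begin and end toggle an InRange flag and swap the Cube's material between active and inactive looks.
; While in range, every Tick spawns a flame actor at the Arrow's transform, alternating between the Fire and Fire1 classes.
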(event `self.ReceiveTick`
  (params (DeltaSeconds :type "Float (single-precision)"))
  (if (`self.In Range`)
    (if (`self.SpawnFlame`)
      (`|SpawnActorFromClass` "/Game/NathansContent/Blueprints/Traps/Fire.Fire_C" (`SceneComponent.K2_GetComponentToWorld` (`self.Arrow`)) "AlwaysSpawn" "OverrideRootScale" null null)
      (set `self.SpawnFlame` false)
      (else
        (`|SpawnActorFromClass` "/Game/NathansContent/Blueprints/Traps/Fire1.Fire1_C" (`SceneComponent.K2_GetComponentToWorld` (`self.Arrow`)) "AlwaysSpawn" "OverrideRootScale" null null)
        (set `self.SpawnFlame` true)))))

(event `self.Box.OnComponentBeginOverlap`
  (params (OverlappedComponent :type "PrimitiveComponent Object Reference") (OtherActor :type "Actor Object Reference") (OtherComp :type "PrimitiveComponent Object Reference") (OtherBodyIndex :type Integer) (bFromSweep :type Boolean) (SweepResult :type "HitResult Structure (by ref)"))
  (cast `/Game/2DTopDownControllerStuff/TopDownCharacter` OtherActor)
  (set `self.In Range` true)
  (`PrimitiveComponent.SetMaterial` (`self.Cube`) 0 "/Game/MaxContent/Sprites/Traps/FireTrap_active2_Mat.FireTrap_active2_Mat"))

(event `self.Box.OnComponentEndOverlap`
  (params (OverlappedComponent :type "PrimitiveComponent Object Reference") (OtherActor :type "Actor Object Reference") (OtherComp :type "PrimitiveComponent Object Reference") (OtherBodyIndex :type Integer))
  (cast `/Game/2DTopDownControllerStuff/TopDownCharacter` OtherActor)
  (set `self.In Range` false)
  (`PrimitiveComponent.SetMaterial` (`self.Cube`) 0 "/Game/MaxContent/Sprites/Traps/FireTrap_unactive_Mat.FireTrap_unactive_Mat"))

(fn `UserConstructionScript`)