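; Fire jet trap that switches itself on and off at random intervals.
; While active, Tick spawns alternating Fire and Fire1 actors at the Arrow's transform every frame.
; Tick also rerolls the idle and burn durations and drives latent Delays through the IsActive and CanActivate flags.
; Each switch swaps the Cube's material to show whether the trap is active.
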(event `self.ReceiveTick`
  (params (DeltaSeconds :type "Float (single-precision)"))
  (`|ExecutionSequence`
    (:`then_0`
      (if (`self.IsActive`)
        (if (`self.SpawnFlame`)
          (`|SpawnActorFromClass` "/Game/NathansContent/Blueprints/Traps/Fire.Fire_C" (`SceneComponent.K2_GetComponentToWorld` (`self.Arrow`)) "AlwaysSpawn" "OverrideRootScale" null null)
          (set `self.SpawnFlame` false)
          (else
            (`|SpawnActorFromClass` "/Game/NathansContent/Blueprints/Traps/Fire1.Fire1_C" (`SceneComponent.K2_GetComponentToWorld` (`self.Arrow`)) "AlwaysSpawn" "OverrideRootScale" null null)
            (set `self.SpawnFlame` true)))))
    (:`then_1`
      (set `self.Delay` (`KismetMathLibrary.RandomFloatInRange` 2.0 20.0))
      (set `self.OnDelay` (`KismetMathLibrary.RandomFloatInRange` 2.0 10.0)))
    (:`then_2`
      (if (`self.CanActivate`)
        (set `self.CanActivate` false)
        (`KismetSystemLibrary.Delay` (`self.Delay`))
        (set `self.IsActive` true)
        (`PrimitiveComponent.SetMaterial` (`self.Cube`) 0 "/Game/MaxContent/Sprites/Traps/FireTrap_active1_Mat.FireTrap_active1_Mat")
        (elif (`self.IsActive`)
          (`KismetSystemLibrary.Delay` (`self.OnDelay`))
          (set `self.IsActive` false)
          (set `self.CanActivate` true)
          (`PrimitiveComponent.SetMaterial` (`self.Cube`) 0 "/Game/MaxContent/Sprites/Traps/FireTrap_unactive_Mat.FireTrap_unactive_Mat"))))))

(fn `UserConstructionScript`)