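; Destroyer is a trap actor that removes cars that enter its box volume.
; When the Box component begins overlapping an actor, a Sequence node tries a separate cast for each of five car classes, Car and Car1 through Car4.
; Any successful cast destroys that car, and the graph does nothing for other actors.
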(event `self.Box.OnComponentBeginOverlap`
  (params (OverlappedComponent :type "PrimitiveComponent Object Reference") (OtherActor :type "Actor Object Reference") (OtherComp :type "PrimitiveComponent Object Reference") (OtherBodyIndex :type Integer) (bFromSweep :type Boolean) (SweepResult :type "HitResult Structure (by ref)"))
  (`|ExecutionSequence`
    (:`then_0`
      (bind _ascar (cast `/Game/NathansContent/Blueprints/Traps/Car` OtherActor))
      (`self.K2_DestroyActor` _ascar))
    (:`then_1`
      (bind _ascar_1 (cast `/Game/NathansContent/Blueprints/Traps/Car1` OtherActor))
      (`self.K2_DestroyActor` _ascar_1))
    (:`then_2`
      (bind _ascar_2 (cast `/Game/NathansContent/Blueprints/Traps/Car2` OtherActor))
      (`self.K2_DestroyActor` _ascar_2))
    (:`then_3`
      (bind _ascar_3 (cast `/Game/NathansContent/Blueprints/Traps/Car3` OtherActor))
      (`self.K2_DestroyActor` _ascar_3))
    (:`then_4`
      (bind _ascar_4 (cast `/Game/NathansContent/Blueprints/Traps/Car4` OtherActor))
      (`self.K2_DestroyActor` _ascar_4))))

(fn `UserConstructionScript`)