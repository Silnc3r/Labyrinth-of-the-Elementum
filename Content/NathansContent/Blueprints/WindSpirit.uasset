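; WindSpirit is an AI pawn that wanders the navmesh and switches to chasing when it sees a pawn.
; PawnSensing sightings set the chase flags and issue a move toward player controller 0, while a retriggerable delay clears the sensing flag once sightings stop.
; Tick drops the chase after a short grace delay, then, when not chasing, moves to random reachable points around itself at random intervals.
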(event `self.ReceiveBeginPlay`)

(event `self.PawnSensing.OnSeePawn`
  (params (Pawn :type "Pawn Object Reference"))
  (`|ExecutionSequence`
    (:`then_0`
      (set `self.IsSensingPawn` true)
      (set `self.IsChasing` true)
      (`|AIMoveTo` self (0.0 0.0 0.0) (`GameplayStatics.GetPlayerController` 0)))
    (:`then_1`
      (`KismetSystemLibrary.RetriggerableDelay` 0.6)
      (set `self.IsSensingPawn` false))))

(event `self.ReceiveTick`
  (params (DeltaSeconds :type "Float (single-precision)"))
  (`|ExecutionSequence`
    (:`then_0`
      (if (not (`self.IsSensingPawn`))
        (`KismetSystemLibrary.Delay` 0.4)
        (if (not (`self.IsSensingPawn`))
          (set `self.IsChasing` false))))
    (:`then_1`
      (if (not (`self.IsChasing`))
        (`KismetSystemLibrary.Delay` (`KismetMathLibrary.RandomFloatInRange` 2.0 5.0))
        (`|AIMoveTo` self (`NavigationSystemV1.K2_GetRandomReachablePointInRadius` (`self.K2_GetActorLocation`) 1500.0 null null) null)))))

(fn `UserConstructionScript`)