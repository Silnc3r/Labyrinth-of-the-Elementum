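; Pickup actor that grants the TopDownCharacter a random power-up when touched.
; Its sphere's begin-overlap casts the other actor to TopDownCharacter, destroys the pickup and rolls a random integer.
; The roll picks one of three effects: refilling health to max, adding a life, or calling the character's SpeedBoost.
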(event `self.Sphere.OnComponentBeginOverlap`
  (params (OverlappedComponent :type "PrimitiveComponent Object Reference") (OtherActor :type "Actor Object Reference") (OtherComp :type "PrimitiveComponent Object Reference") (OtherBodyIndex :type Integer) (bFromSweep :type Boolean) (SweepResult :type "HitResult Structure (by ref)"))
  (bind _astop_down_character (cast `/Game/2DTopDownControllerStuff/TopDownCharacter` OtherActor))
  (`self.K2_DestroyActor`)
  (set `self.PowerUp` (`KismetMathLibrary.RandomIntegerInRange` 1 3))
  (if (== (`self.PowerUp`) 1)
    (set `/Game/2DTopDownControllerStuff/TopDownCharacter.Health` (`/Game/2DTopDownControllerStuff/TopDownCharacter.MaxHealth` _astop_down_character) _astop_down_character)
    (elif (== (`self.PowerUp`) 2)
      (set `/Game/2DTopDownControllerStuff/TopDownCharacter.LifeCount` (+ (`/Game/2DTopDownControllerStuff/TopDownCharacter.LifeCount` _astop_down_character) 1) _astop_down_character)
      (elif (== (`self.PowerUp`) 3)
        (`/Game/2DTopDownControllerStuff/TopDownCharacter.SpeedBoost` _astop_down_character)))))

(fn `UserConstructionScript`)