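; Game manager for a top-down game that tracks the game state and switches UI between main menu, pause and running.
; Init has TopDownGameMode create the UI, then requests the MainMenu state.
; SetState acts only on a state change: it hides UI, shows the matching menu and toggles the mouse cursor.
; Each entry into Running creates a new health bar widget and adds it to the viewport.
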(fn `Init`
  (bind _astop_down_game_mode (cast `/Game/TopDownBP/Blueprints/TopDownGameMode` (`GameplayStatics.GetGameMode`)))
  (`/Game/TopDownBP/Blueprints/TopDownGameMode.CreateUI` _astop_down_game_mode)
  (`self.SetState` "NewEnumerator6"))

(fn `SetState`
  (params (NewState :type "/Game/Henry-Content/Menus/MyGameStates Enum" :default "NewEnumerator0"))
  (if (!= NewState (`self.Current Game State`))
    (bind _output_get (set `self.Current Game State` NewState))
    (switch `/Game/Henry-Content/Menus/MyGameStates` _output_get
      (:`NewEnumerator0`
        (`/Game/Henry-Content/Blueprints/HenryFunctionLibrary.ShowMouse` false)
        (`/Game/Henry-Content/Blueprints/HenryFunctionLibrary.HideUI`)
        ;[1 1 1] Max - Health Bar
        (bind _returnvalue (`|CreateWidget` "/Game/MaxContent/UI/HealthBar.HealthBar_C"))
        (bind _output_get_2 (set `self.HealthWidget` _returnvalue))
        (`UserWidget.AddToViewport` _output_get_2 0))
      (:`NewEnumerator3`
        ;[1 1 1] Henry
        ;;[1 1 1] Pause menu
        (`/Game/Henry-Content/Blueprints/HenryFunctionLibrary.HideUI`)
        (`Widget.SetVisibility` (`self.Widget_PauseMenu`) "Visible")
        (`/Game/Henry-Content/Blueprints/HenryFunctionLibrary.ShowMouse` true))
      (:`NewEnumerator6`
        ;;[1 1 1] Main Menu
        (`/Game/Henry-Content/Blueprints/HenryFunctionLibrary.HideUI`)
        (`Widget.SetVisibility` (`self.Widget_MainMenu`) "Visible")
        (`/Game/Henry-Content/Blueprints/HenryFunctionLibrary.ShowMouse` true)))))

(fn `UserConstructionScript`)